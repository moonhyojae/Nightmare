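; BP_FirstMonster is an enemy that chases the player and periodically shoots at them once the player's Y position passes zero.
; Tick updates player direction and drives a state switch between following and attacking, with the attack timer gated by the monster's Y position.
; Attacking pauses movement, then spawns a BP_Bullet from Arrow1 after a delay.
; Capsule contact with BP_Player shows WBP_Menu and destroys the player; the distance-based hold logic is disconnected.
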(event OnComponentHit(CapsuleComponent)
  (params (HitComponent :type Primitive%20Component%20Object%20Reference) (OtherActor :type Actor%20Object%20Reference) (OtherComp :type Primitive%20Component%20Object%20Reference) (NormalImpulse :type Vector :default "0, 0, 0") (Hit :type Hit%20Result%20Structure%20%28by%20ref%29))
  ;[1 1 1] 플레이어와 충돌시 파괴
  (bind _asbp_player (Utilities|Casting|CastToBP_Player OtherActor))
  (CallFunction|EndGame)
  (Actor|DestroyActor _asbp_player))

(event EventBeginPlay)

(event EventTick
  (params (DeltaSeconds :type Float%20%28single-precision%29))
  (CallFunction|DisandDirtoPlayer)
  (if (Utilities|IsValid (Game|GetPlayerCharacter 0))
    (if (> (.y (Transformation|GetActorLocation (Game|GetPlayerCharacter 0))) 0.0)
      (switch Utilities|FlowControl|Switch|SwitchonMonsterState (Variables|Default|GetCurstate)
        (:NewEnumerator0
          ;[1 1 1] 일정 시간에 한번씩 플레이어를 공격
          (if (> (.y (Transformation|GetActorLocation)) -2e+02)
            (Variables|Default|SetCurrentTime (+ DeltaSeconds (Variables|Default|GetCurrentTime)))
            (if (> (Variables|Default|GetCurrentTime) (Variables|Default|GetCreateTime))
              (Variables|Default|SetCurstate "NewEnumerator1")
              (Variables|Default|SetIsAttacking true)
              (Variables|Default|SetCurrentTime 0.0)
              (else
                (Pawn|Input|AddMovementInput (Variables|Default|GetDirToPlayerCharac) 1.0 false :!label _label)))
            (else
              (goto _label))))
        (:NewEnumerator1
          ;[1 1 1] 공격상태일때 공격하고 아닐시 플레이어를 쫒아감
          (if (Variables|Default|GetIsAttacking)
            (Variables|Default|SetCurrentTime (+ DeltaSeconds (Variables|Default|GetCurrentTime)))
            (if (> (Variables|Default|GetCurrentTime) (Variables|Default|GetStopTime))
              (Variables|Default|SetCurrentTime 0.0)
              (Variables|Default|SetIsAttacking false)
              (Game|SpawnActorfromClass "/Game/Buleprints/BP_Bullet.BP_Bullet_C" (Transformation|GetWorldTransform (Variables|Default|GetArrow1)) "AlwaysSpawn" 0 0))
            (else
              (Variables|Default|SetCurstate "NewEnumerator0"))))))))

(fn ConstructionScript)

(fn DisandDirtoPlayer
  (bind _returnvalue (Game|GetPlayerCharacter 0))
  (bind _returnvalue_2 (Transformation|GetActorLocation))
  (bind _returnvalue_3 (Transformation|GetActorLocation _returnvalue))
  (bind _returnvalue_4 (- _returnvalue_3 _returnvalue_2))
  (bind (_x _y _z) (Math|Vector|BreakVector _returnvalue_4))
  (bind _returnvalue_5 (Math|Vector|MakeVector _x _y _z))
  ;[1 1 1] 플레이어와 몬스터의 거리 및 방향 저장
  (if (Utilities|IsValid _returnvalue)
    (Variables|Default|SetDistancePlayerCharac (Math|Vector|VectorLength _returnvalue_5))
    (Variables|Default|SetDirToPlayerCharac (Math|Vector|Normalize _returnvalue_5))
    (else
      (Variables|Default|SetDistancePlayerCharac 0.0)
      (Variables|Default|SetDirToPlayerCharac "0, 0, 0"))))

(fn EndGame
  (Variables|/Script/Engine.PlayerController|SetbShowMouseCursor (Game|GetPlayerController 0) true)
  (bind _returnvalue (UserInterface|CreateWidget "/Game/UI/WBP_Menu.WBP_Menu_C"))
  (UserInterface|Viewport|AddtoViewport _returnvalue 0))