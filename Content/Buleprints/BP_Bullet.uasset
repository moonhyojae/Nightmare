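; BP_Bullet is a projectile that flies in a straight line toward where the player stood when it spawned.
; BeginPlay stores that direction, and Tick moves the bullet along it by Speed and delta time with a swept move.
; Sphere hits always destroy the bullet, also destroying any BP_Cube struck but leaving the player intact.
; EndGame shows the cursor and WBP_Menu, but nothing here calls it.
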(event OnComponentHit(Sphere)
  (params (HitComponent :type Primitive%20Component%20Object%20Reference) (OtherActor :type Actor%20Object%20Reference) (OtherComp :type Primitive%20Component%20Object%20Reference) (NormalImpulse :type Vector :default "0, 0, 0") (Hit :type Hit%20Result%20Structure%20%28by%20ref%29))
  ;[1 1 1] 충돌한 물체가 플레이어일시 GameOver 위젯을 띄우고 플레이어와 불렛 파괴, 상자일시 상자와 불렛 파괴
  (Utilities|Casting|CastToBP_Player OtherActor
    (:then
      (Actor|DestroyActor))
    (:CastFailed
      (bind _asbp_cube (Utilities|Casting|CastToBP_Cube OtherActor)
        (:then
          (Actor|DestroyActor _asbp_cube)
          (Actor|DestroyActor))
        (:CastFailed
          (Actor|DestroyActor))))))

(event EventBeginPlay
  ;[1 1 1] 플레이어(타겟)과 총알의 시작 벡터
  (Variables|Default|SetDirection (- (Transformation|GetActorLocation (Game|GetPlayerCharacter 0)) (Transformation|GetActorLocation))))

(event EventTick
  (params (DeltaSeconds :type Float%20%28single-precision%29))
  ;[1 1 1] 해당 벡터로 발사
  (Transformation|SetActorLocation (+ (Transformation|GetActorLocation) (* (* (Math|Vector|Normalize (Variables|Default|GetDirection)) (Variables|Default|GetSpeed)) DeltaSeconds)) true false))

(fn ConstructionScript)

(fn EndGame
  (Variables|/Script/Engine.PlayerController|SetbShowMouseCursor (Game|GetPlayerController 0) true)
  (bind _returnvalue (UserInterface|CreateWidget "/Game/UI/WBP_Menu.WBP_Menu_C"))
  (UserInterface|Viewport|AddtoViewport _returnvalue 0))