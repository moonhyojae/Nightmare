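; BP_Camera_2 is a follow camera actor that trails the player character along the Y and Z axes while keeping its X position fixed.
; BeginPlay stores the initial offset between the camera and player character 0.
; Tick lerps toward the player's location plus that offset, using DeltaSeconds times Smooth as alpha, and holds position when the player is invalid.
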(event EventBeginPlay
  ;[1 1 1] 플레이어와 카메라의 간격
  (Variables|Default|SetOffset (- (Transformation|GetActorLocation) (Transformation|GetActorLocation (Game|GetPlayerCharacter 0)))))

(event EventTick
  (params (DeltaSeconds :type Float%20%28single-precision%29))
  (bind _returnvalue (Game|GetPlayerCharacter 0))
  (bind _returnvalue_2 (Transformation|GetActorLocation))
  (bind _offset (Variables|Default|GetOffset))
  (bind _smooth (Variables|Default|GetSmooth))
  (bind _returnvalue_3 (Transformation|GetActorLocation _returnvalue))
  (bind _returnvalue_4 (* DeltaSeconds _smooth))
  (bind _returnvalue_5 (+ _returnvalue_3 _offset))
  (bind _returnvalue_6 (Math|Vector|Lerp(Vector) _returnvalue_2 _returnvalue_5 _returnvalue_4))
  ;[1 1 1] 카메라가 플레이어를 따라감
  (if (Utilities|IsValid _returnvalue)
    (Transformation|SetActorLocation (Math|Vector|MakeVector (.x (Transformation|GetActorLocation)) (.y _returnvalue_6) (.z _returnvalue_6)) false false)
    (else
      (Transformation|SetActorLocation (Transformation|GetActorLocation) false false))))

(fn ConstructionScript)