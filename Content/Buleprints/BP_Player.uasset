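; BP_Player is the player character Blueprint, handling movement, jumping, ladder climbing, camera setup and death.
; On begin play it shows a key UI and switches the view to a "Cam"-tagged actor; movement follows fixed world axes.
; Interact toggles climbing near ladders, using Flying mode and snapping to the first BP_Ladder found.
; A BP_Bullet hit plays a death animation and opens the menu after a delay; P triggers ragdoll.
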(event OnComponentHit(CapsuleComponent)
  (params (HitComponent :type Primitive%20Component%20Object%20Reference) (OtherActor :type Actor%20Object%20Reference) (OtherComp :type Primitive%20Component%20Object%20Reference) (NormalImpulse :type Vector :default "0, 0, 0") (Hit :type Hit%20Result%20Structure%20%28by%20ref%29))
  (Utilities|Casting|CastToBP_Bullet OtherActor)
  (Components|Animation|PlayAnimation (Variables|Character|GetMesh) "/Game/Mesh/Player/Animations/Death.Death" false)
  (Components|Activation|Deactivate (Variables|Character|GetCharacterMovement))
  (Components|DestroyComponent (Variables|Collision|GetCapsuleComponent))
  (Utilities|FlowControl|Delay 2.0)
  (CallFunction|EndGame))

(event EventBeginPlay
  ;[1 1 1] 키 입력 UI
  (bind _returnvalue (UserInterface|CreateWidget "/Game/UI/WBP_KeyUI.WBP_KeyUI_C"))
  (UserInterface|Viewport|AddtoViewport _returnvalue 0)
  (Collision|SetCollisionEnabled (Variables|Default|GetPlayerHand) "NoCollision")
  ;[1 1 1] 카메라 설정
  (bind _outactors (Actor|GetAllActorswithTag "Cam"))
  (Game|Player|SetViewTargetwithBlend (Game|GetPlayerController 0) (Utilities|Array|Get(acopy) _outactors) 0.0 "VTBlend_Linear" 0.0 false))

(event Collision|EventActorBeginOverlap
  (params (OtherActor :type Actor%20Object%20Reference)))

(event EventTick
  (params (DeltaSeconds :type Float%20%28single-precision%29)))

(event Input|ActionEvents|InputActionJump
  (params (Key :type Key%20Structure :default "None"))
  (:Pressed
    (Character|Jump)))

(event Input|ActionEvents|InputActioninteract
  (params (Key :type Key%20Structure :default "None"))
  ;[1 1 1] interact 입력시 플레이어가 사다리에 있으면 사다리에서 내림. 없으면 사다리에 올라탐
  (:Pressed
    (if (Variables|Default|GetNear%20ladder?)
      (if (Variables|Default|GetOn%20ladder?)
        (Variables|Default|SetOn%20ladder? false)
        (Pawn|Components|CharacterMovement|SetMovementMode (Variables|Character|GetCharacterMovement) "MOVE_Walking" 0)
        (else
          (Variables|Default|SetOn%20ladder? true))))))

(event Input|AxisEvents|InputAxisForward/Backward
  (params (AxisValue :type Float%20%28single-precision%29))
  (bind _returnvalue (Transformation|GetActorRotation))
  ;[1 1 1] 플레이어가 사다리에 있으면 forward/backward 입력시 위아래로 이동
  ;;[1 1 1] 이동
  (if (Variables|Default|GetOn%20ladder?)
    (Pawn|Components|CharacterMovement|SetMovementMode (Variables|Character|GetCharacterMovement) "MOVE_Flying" 0)
    (Pawn|Input|AddMovementInput (Transformation|GetActorUpVector (Game|GetPlayerCharacter 0)) AxisValue false)
    (bind _outactors (Actor|GetAllActorsOfClass "/Game/Buleprints/BP_Ladder.BP_Ladder_C"))
    (Transformation|SetActorRotation (Math|Rotator|MakeRotator (.roll _returnvalue) (.pitch _returnvalue) 0.0))
    (Transformation|SetActorLocation (Math|Vector|MakeVector (- (.x (Transformation|GetActorLocation (Utilities|Array|Get(acopy) _outactors))) 5e+01) (.y (Transformation|GetActorLocation (Utilities|Array|Get(acopy) _outactors))) (.z (Transformation|GetActorLocation))) false false)
    (else
      (Variables|Default|SetOn%20ladder? false)
      (Pawn|Input|AddMovementInput (Math|Vector|GetForwardVector "0, 0, 0") AxisValue false))))

(event Input|AxisEvents|InputAxisLeft/Right
  (params (AxisValue :type Float%20%28single-precision%29))
  ;[1 1 1] 플레이어가 사다리에 있으면 forward/backward 입력시 위아래로 이동
  ;;[1 1 1] 이동
  (if (not (Variables|Default|GetOn%20ladder?))
    (Pawn|Input|AddMovementInput (Math|Vector|GetRightVector "0, 0, 0") AxisValue false)))

(event Input|KeyboardEvents|P
  (params (Key :type Key%20Structure :default "None"))
  (:Pressed
    (CallFunction|Ragdoll/Death)))

(fn ConstructionScript)

(fn Ragdoll/Death
  (Physics|SetSimulatePhysics (Variables|Character|GetMesh) true)
  (Pawn|Components|CharacterMovement|DisableMovement (Variables|Character|GetCharacterMovement)))

(fn EndGame
  (Variables|/Script/Engine.PlayerController|SetbShowMouseCursor (Game|GetPlayerController 0) true)
  (bind _returnvalue (UserInterface|CreateWidget "/Game/UI/WBP_Menu.WBP_Menu_C"))
  (UserInterface|Viewport|AddtoViewport _returnvalue 0))