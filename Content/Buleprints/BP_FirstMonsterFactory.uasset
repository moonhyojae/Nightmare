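; BP_FirstMonsterFactory is a spawner actor that creates a BP_FirstMonster at its own transform when the player reaches a trigger line.
; Each Tick, it checks whether player character 0's world Y lies strictly inside a narrow band just above zero, though the node comment cites 600–605.
; A MonsterCnt counter gates spawning below one and is never decremented here, so this graph alone does not respawn the monster.
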(event EventBeginPlay)

(event Collision|EventActorBeginOverlap
  (params (OtherActor :type Actor%20Object%20Reference)))

(event EventTick
  (params (DeltaSeconds :type Float%20%28single-precision%29))
  (bind _returnvalue (Game|GetPlayerCharacter 0))
  (if (Utilities|IsValid _returnvalue)
    (if (and (> (.y (Transformation|GetActorLocation _returnvalue)) 0.0) (< (.y (Transformation|GetActorLocation (Game|GetPlayerCharacter 0))) 5.0))
      ;[1 1 1] 몬스터가 없으면 소환
      (if (not (>= (Variables|Default|GetMonsterCnt) 1))
        (Variables|Default|SetMonsterCnt (+ (Variables|Default|GetMonsterCnt) 1))
        (Game|SpawnActorfromClass "/Game/Buleprints/BP_FirstMonster.BP_FirstMonster_C" (Transformation|GetActorTransform) "Undefined" 0 0)))))

(fn ConstructionScript)