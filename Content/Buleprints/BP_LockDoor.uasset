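; BP_LockDoor is a locked door that the player can open with an input action when holding a key.
; Hitting its Box with BP_Player stores the player, enables input and opens a Gate; the disable-and-close branch is unconnected.
; A FlipFlop, with only A wired, plays a timeline that lerps door yaw from closed to open angle.
; The door sound spawns on every timeline update.
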(event OnComponentHit(Box)
  (params (HitComponent :type Primitive%20Component%20Object%20Reference) (OtherActor :type Actor%20Object%20Reference) (OtherComp :type Primitive%20Component%20Object%20Reference) (NormalImpulse :type Vector :default "0, 0, 0") (Hit :type Hit%20Result%20Structure%20%28by%20ref%29))
  ;[1 1 1] Open the door 버튼 입력시 열쇠가 있으면 문을 열고 없으면 안 엶
  (bind _asbp_player (Utilities|Casting|CastToBP_Player OtherActor))
  (Input|EnableInput (Game|GetPlayerController 0))
  (Utilities|FlowControl|Gate true) ; enters at Open
)

(event EventBeginPlay)

(event Collision|EventActorBeginOverlap
  (params (OtherActor :type Actor%20Object%20Reference)))

(event EventTick
  (params (DeltaSeconds :type Float%20%28single-precision%29)))

(event Input|ActionEvents|InputActionOpenthedoor
  (params (Key :type Key%20Structure :default "None"))
  ;[1 1 1] Open the door 버튼 입력시 열쇠가 있으면 문을 열고 없으면 안 엶
  (:Pressed
    (if (Variables|/Game/Buleprints/BP_Player.BP_Player_C|GetHas%20key? (stale OnComponentHit(Box) _asbp_player))
      (Utilities|FlowControl|Gate true
        (:Exit
          ;[1 1 1] 문 열고 닫는 모션
          (Utilities|FlowControl|FlipFlop
            (:A
              (bind _doortrack (Timeline|Opem/Close%20Door Play)
                (:Update
                  (Transformation|SetRelativeRotation (Variables|Components|GetDoor) (Math|Rotator|MakeRotator 0.0 0.0 (Math|Float|Lerp (Variables|Default|GetClosed%20Angle) (Variables|Default|GetOpen%20Angle) _doortrack)) false false)
                  ;[1 1 1] 문 열리는 효과음 넣기
                  (Audio|SpawnSoundatLocation "/Game/Sound/door_Cue.door_Cue" (Transformation|GetActorLocation) "0, 0, 0" 1.0 1.0 0.0 0 0))))))))))

(fn ConstructionScript)